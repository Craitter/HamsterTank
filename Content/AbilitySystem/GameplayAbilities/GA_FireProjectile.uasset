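; Gameplay Ability that fires a projectile by spawning BP_Projectile from the avatar actor.
; GetProjectileTransform finds the avatar's ProjectileOriginComponent, caches it along with the avatar, and returns its world transform as the spawn point.
; On activation, a successful commit spawns the projectile with the avatar as owner and ends the ability once the projectile is valid.
; A failed commit cancels the ability.
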(event `self.K2_ActivateAbility`
  (bind _spawntransform (`self.GetProjectileTransform`))
  (bind _returnvalue (`self.K2_CommitAbility`))
  (if _returnvalue
    (bind _returnvalue_2 (`|SpawnActorFromClass` "/Game/Actors/Projectile/BP_Projectile.BP_Projectile_C" _spawntransform "AlwaysSpawn" "MultiplyWithRoot" (`self.OwningActor`) null))
    (bind _output_get (set `self.Projectile` _returnvalue_2))
    (`/Engine/EditorBlueprintResources/StandardMacros.IsValid` _output_get
      (:`Is Valid`
        (`self.K2_EndAbility`)))
    (else
      (`self.K2_CancelAbility`))))

(fn `GetProjectileTransform`
  (returns (SpawnTransform :type "Transform Structure"))
  (`/Engine/EditorBlueprintResources/StandardMacros.IsValid` (`self.ProjectileOrigin`)
    (:`Is Valid`
      _)
    (:`Is Not Valid`
      (bind _output_get (set `self.OwningActor` (`self.GetAvatarActorFromActorInfo`)))
      (`/Engine/EditorBlueprintResources/StandardMacros.IsValid` _output_get
        (:`Is Valid`
          (bind _output_get_2 (set `self.ProjectileOrigin` (`Actor.GetComponentByClass` (`self.OwningActor`) "/Script/HamsterTank.ProjectileOriginComponent")))
          (`/Engine/EditorBlueprintResources/StandardMacros.IsValid` _output_get_2
            (:`Is Valid`
              _)
            (:`Is Not Valid`
              _))))))
  (return (`SceneComponent.K2_GetComponentToWorld` (`self.ProjectileOrigin`))))